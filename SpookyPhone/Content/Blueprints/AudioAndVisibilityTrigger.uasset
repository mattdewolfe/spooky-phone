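; AudioAndVisibilityTrigger is a one-shot overlap trigger that hides a group of objects and plays a positioned sound.
; An actor overlap calls StartEvent on itself, and the EventUpdate handler does the work, guarded by IsTriggered.
; It casts the player pawn to SpookyPawn to turn off the chosen hideable group's visibility, then plays the configured sound at AudioPosition.
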(event EventEventUpdate
  (if (not (Variables|Default|GetisTriggered))
    (Variables|Default|SetisTriggered true)
    (bind _asspooky_pawn (Utilities|Casting|CastToSpookyPawn (Game|Player|GetPlayerPawn 0)))
    (Class|SpookyPawn|SetHideableGroupVisibility _asspooky_pawn false (Math|Conversions|ToByte(Integer) (Variables|Default|GetGroupToToggle)))
    (Audio|PlaySoundatLocation (Variables|Default|GetAudioToPlay) (Variables|Default|GetAudioPosition))))

(event EventBeginPlay)

(event EventActorBeginOverlap
  (params (OtherActor :type Actor%20Object%20Reference))
  (Class|EventBlueprintFunctionLibrary|StartEvent self))

(event EventTick
  (params (DeltaSeconds :type Float%20%28single-precision%29)))

(fn ConstructionScript)