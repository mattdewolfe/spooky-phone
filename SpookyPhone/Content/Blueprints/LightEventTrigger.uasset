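; Overlap-triggered actor for a timed light event that can flicker a referenced Lamp.
; The first overlap calls StartEvent, starts a looping OnTimedEvent timer and resets Count to CallCount.
; Each tick of that timer decrements and prints Count, while a separate EventUpdate event triggers the flicker.
; The zero-count check that clears the timer and calls EndEvent is unconnected, so the countdown never stops itself.
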(event EventEventUpdate
  (Default|Flicker (Variables|Default|GetLamp)))

(event EventBeginPlay)

(event EventActorBeginOverlap
  (params (OtherActor :type Actor%20Object%20Reference))
  (bind _self self)
  (if (not (Variables|Default|GetbEventStarted))
    (Class|EventBlueprintFunctionLibrary|StartEvent _self)
    (Utilities|Time|SetTimerbyFunctionName _self "OnTimedEvent" (Variables|Default|GetTime) true)
    (Variables|Default|SetbEventStarted true)
    (CallFunction|ResetCount)))

(event EventTick
  (params (DeltaSeconds :type Float%20%28single-precision%29)))

(fn ConstructionScript)

(fn OnTimedEvent
  (bind _output_get (Variables|Default|SetCount (- (Variables|Default|GetCount) 1)))
  (Development|PrintString (Utilities|String|ToString(Integer) _output_get)))

(fn ResetCount
  (Variables|Default|SetCount (Variables|Default|GetCallCount)))