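; Trigger actor that sends the game to the GameOverWin level when the victory condition is met inside it.
; Begin and end overlap set an IsPlayerInside flag for any actor, with no check that it is the player.
; While the flag is set, Tick casts the player character to SpookyPawn and polls CheckVictory, opening the win level when it returns true.
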(event EventBeginPlay)

(event EventActorBeginOverlap
  (params (OtherActor :type Actor%20Object%20Reference))
  (Variables|Default|SetisPlayerInside true))

(event EventTick
  (params (DeltaSeconds :type Float%20%28single-precision%29))
  (if (Variables|Default|GetisPlayerInside)
    (bind _asspooky_pawn (Utilities|Casting|CastToSpookyPawn (Game|GetPlayerCharacter 0)))
    (bind _returnvalue (Class|SpookyPawn|CheckVictory _asspooky_pawn))
    (if _returnvalue
      (Game|OpenLevel(byName) "GameOverWin"))))

(event EventActorEndOverlap
  (params (OtherActor :type Actor%20Object%20Reference))
  (Variables|Default|SetisPlayerInside false))

(fn ConstructionScript)