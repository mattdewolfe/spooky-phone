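; A trigger actor that plays its assigned sound once, at its own location.
; Actor overlap calls StartEvent on itself, with no filter on the overlapping actor.
; The EventUpdate handler checks and sets a Triggered flag, so only its first call runs PlaySoundOnce.
; PlaySoundOnce plays TriggeredSound at the actor's transform origin, and nothing in these graphs resets the flag.
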(event EventEventUpdate
  ;[1 1 1] Comment
  (if (not (Variables|Default|GetbTriggered))
    (Variables|Default|SetbTriggered true)
    (CallFunction|PlaySoundOnce)))

(event EventBeginPlay)

(event EventActorBeginOverlap
  (params (OtherActor :type Actor%20Object%20Reference))
  ;[1 1 1] Event Start
  (Class|EventBlueprintFunctionLibrary|StartEvent self))

(event EventTick
  (params (DeltaSeconds :type Float%20%28single-precision%29)))

(fn ConstructionScript)

(fn PlaySoundOnce
  (Audio|PlaySoundatLocation (Variables|Default|GetTriggered%20Sound) (Math|Transform|TransformLocation (Transformation|GetActorTransform) "0, 0, 0")))