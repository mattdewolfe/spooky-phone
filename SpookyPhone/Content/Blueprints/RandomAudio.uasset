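; RandomAudio is an actor Blueprint that plays a random sound at its own location on a repeating timer.
; Tick accumulates elapsed time, and once it exceeds the interval set in the construction script, it picks a random entry from an audio array, plays it and resets the timer.
; The construction script fixes that interval, and the overlap event is unused.
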(event EventBeginPlay
  (Variables|Default|SetTimeOfLastAudio 0.0))

(event EventActorBeginOverlap
  (params (OtherActor :type Actor%20Object%20Reference)))

(event EventTick
  (params (DeltaSeconds :type Float%20%28single-precision%29))
  (bind _output_get (Variables|Default|SetTimeOfLastAudio (+ DeltaSeconds (Variables|Default|GetTimeOfLastAudio))))
  (Math|Float|CompareFloat _output_get (Variables|Default|GetTimeBetweenAudio)
    (:>
      (Audio|PlaySoundatLocation (Utilities|Array|Get(acopy) (Variables|Default|GetAudioArray) (Math|Random|RandomIntegerinRange 0 (- (Utilities|Array|Length (Variables|Default|GetAudioArray)) 1))) (Transformation|GetActorLocation))
      (Variables|Default|SetTimeOfLastAudio 0.0))))

(fn ConstructionScript
  (Variables|Default|SetTimeBetweenAudio 25.0))