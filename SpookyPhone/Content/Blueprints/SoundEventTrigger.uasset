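; SoundEventTrigger is a trigger actor that plays a one-shot sound when something overlaps it.
; An overlap calls StartEvent on itself, and the EventUpdate event uses a Triggered flag so the sound fires only the first time.
; PlaySoundOnce plays TriggeredSound at the actor's world location.
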(event EventEventUpdate
  ;[1 1 1] Comment
  (if (not (Variables|Default|GetbTriggered))
    (Variables|Default|SetbTriggered true)
    (CallFunction|PlaySoundOnce)))

(event EventActorBeginOverlap
  (params (OtherActor :type Actor%20Object%20Reference))
  ;[1 1 1] Event Start
  (Class|EventBlueprintFunctionLibrary|StartEvent self))

(fn ConstructionScript)

(fn PlaySoundOnce
  (Audio|PlaySoundatLocation (Variables|Default|GettriggeredSound) (Math|Transform|TransformLocation (Transformation|GetActorTransform) "0, 0, 0")))