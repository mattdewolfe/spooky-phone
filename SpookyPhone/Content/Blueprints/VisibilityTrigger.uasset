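; One-shot trigger actor that makes a selected group of hideable objects visible when an actor overlaps it.
; Any overlap calls StartEvent on itself, and the separate EventUpdate handler does the work.
; On its first run, that handler sets a Triggered flag and tells the player's SpookyPawn to show GroupToToggle.
; It only ever sets visibility on, despite the toggle naming.
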(event EventEventUpdate
  ;[1 1 1] Toggle Visibility
  (if (not (Variables|Default|GetTriggered))
    (Variables|Default|SetTriggered true)
    (bind _asspooky_pawn (Utilities|Casting|CastToSpookyPawn (Game|Player|GetPlayerPawn 0)))
    (Class|SpookyPawn|SetHideableGroupVisibility _asspooky_pawn true (Math|Conversions|ToByte(Integer) (Variables|Default|GetGroupToToggle)))))

(event EventActorBeginOverlap
  (params (OtherActor :type Actor%20Object%20Reference))
  ;[1 1 1] Event Start
  (Class|EventBlueprintFunctionLibrary|StartEvent self))

(fn ConstructionScript)